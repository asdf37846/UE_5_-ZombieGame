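; Zombie game mode that runs a wave-based survival loop, starting on BeginPlay.
; SpawnZombies sets the zombie count from CurrentWave, then runs about half that count at each of four spawn locations, though the last loop has no actor class set.
; ZombieKilled decrements ZombiesLeft and at zero calls WaveIncrement, which starts the next wave or prints a win message at MaxWaves.
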(event `self.ReceiveBeginPlay`
  ;[1 1 1] Start Game
  (`self.StartGame`))

(event `StartGame`
  ;[1 1 1] Start Game
  (`self.SpawnZombies`))

(event `SpawnZombies`
  ;[1 1 1] Spawn Zombies
  (bind _output_get (set `self.ZombieTotal` (* (`self.CurrentWave`) 5)))
  (set `self.ZombiesLeft` _output_get)
  (for _index (range 1 (+ _output_get 1))
    (if (== _index (/ (`self.ZombieTotal`) 2))
      (break)
      (else
        (`|SpawnActorFromClass` "/Game/_Main/Zombie/BP_Zombie.BP_Zombie_C" (`self.SpawnLocation3`) "Undefined" "OverrideRootScale" null null))))
  (for _ (range 1 (+ (/ (`self.ZombieTotal`) 2) 1))
    (`|SpawnActorFromClass` "/Game/_Main/Zombie/BP_Zombie.BP_Zombie_C" (`self.SpawnLocation4`) "Undefined" "OverrideRootScale" null null))
  (for _ (range 1 (+ (/ (`self.ZombieTotal`) 2) 1))
    (`|SpawnActorFromClass` "/Game/_Main/Zombie/BP_Zombie.BP_Zombie_C" (`self.SpawnLocation1`) "Undefined" "OverrideRootScale" null null))
  (for _ (range 1 (+ (/ (`self.ZombieTotal`) 2) 1))
    (`|SpawnActorFromClass` "/Game/_Main/Zombie/BP_Zombie.BP_Zombie_C" (`self.SpawnLocation2`) "Undefined" "OverrideRootScale" null null)))

(event `ZombieKilled`
  ;[1 1 1] Zombie killed
  (bind _result (`/Engine/EditorBlueprintResources/StandardMacros.DecrementInt` (`self.ZombiesLeft`))
    (:`  `
      (if (== _result 0)
        (`self.WaveIncrement`)))))

(event `WaveIncrement`
  (if (== (`self.CurrentWave`) (`self.MaxWaves`))
    (`KismetSystemLibrary.PrintString` "Player Win")
    (else
      (`/Engine/EditorBlueprintResources/StandardMacros.IncrementInt` (`self.CurrentWave`)
        (:`  `
          (`self.SpawnZombies`)
          (`KismetSystemLibrary.PrintString` "Next Wave Start"))))))

(fn `UserConstructionScript`)